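; Bp_item is an item Blueprint that shows an interaction prompt while a player is in its interaction zone.
; On zone entry it creates an Interaciton_widget for that player and hosts it in a runtime-added, screen-space widget component without collision.
; GetInteractionText and GetInteractionAttach supply the label and attach point, defaulting to "Interact" and the scene root.
; Leaving the zone destroys the component.
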(event `/Game/bp_interaface/interaction_interface.on interactionzone entered`
  (params (player :type "/Game/AnimStarterPack/Ue4ASP_Character Object Reference"))
  (`self.interaction widget component`
    (:`then`)
    (:`else`
      (bind _returnvalue (`|CreateWidget` "/Game/bp_interaface/interaciton_widget.interaciton_widget_C" (cast `PlayerController` (`Pawn.GetController` player) :!pure true) (`self.Get interaction text`)))
      (bind _returnvalue_2 (`AddComponent|NODE_AddWidgetComponent-0`))
      (bind _output_get (set `self.interaction widget component` _returnvalue_2))
      (`WidgetComponent.SetWidget` _output_get _returnvalue)
      (`WidgetComponent.SetWidgetSpace` _output_get "Screen")
      (`WidgetComponent.SetDrawAtDesiredSize` _output_get true)
      (`PrimitiveComponent.SetCollisionEnabled` _output_get "NoCollision")
      (`SceneComponent.K2_AttachToComponent` _output_get (`self.get interaction attach`) "None" "SnapToTarget" "SnapToTarget" "SnapToTarget" true))))

(event `/Game/bp_interaface/interaction_interface.on interactionzone exited `
  (bind _interaction_widget_component (`self.interaction widget component`)
    (:`then`
      (`ActorComponent.K2_DestroyComponent` _interaction_widget_component))
    (:`else`)))

(fn `get interaction attach`
  (returns (`attach component` :type "SceneComponent Object Reference"))
  (return (`self.DefaultSceneRoot`)))

(fn `Get interaction text`
  (returns (text :type Text))
  (return "Interact"))

(fn `UserConstructionScript`)