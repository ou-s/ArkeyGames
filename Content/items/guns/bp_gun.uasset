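; Base gun item that a player can pick up through interaction and fire.
; A Droped/Equiped state toggles mesh physics and collision on the mesh and pickup sphere, starting dropped and becoming equipped on pickup.
; Fire spawns an actor at the muzzle socket, aimed at a far point along the camera's forward vector, plus a muzzle effect.
; Velocity and fire-rate getters return placeholder defaults, with no projectile class set here.
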(event `self.ReceiveBeginPlay`
  (`self.set gun state` "NewEnumerator0"))

(event `/Game/bp_interaface/interaction_interface.on iteraction `
  (params (player :type "/Game/AnimStarterPack/Ue4ASP_Character Object Reference"))
  (`/Game/AnimStarterPack/Ue4ASP_Character.PIck up GUn` player self)
  (`self.set gun state` "NewEnumerator1"))

(fn `Droped`
  (`self.set gun state` "NewEnumerator0"))

(fn `equpied`
  (set `self.Gun State` "NewEnumerator1"))

(fn `Fire`
  (params (`player camera` :type "CameraComponent Object Reference"))
  (bind _returnvalue (`SceneComponent.GetSocketLocation` (`self.SkeletalMesh`) "b_gun_muzzleflash"))
  (`|ExecutionSequence`
    (:`then_0`
      (`|SpawnActorFromClass` "/Game/bullet/bp_bullet.bp_bullet_C" (`KismetMathLibrary.MakeTransform` _returnvalue (`self.K2_GetActorRotation`)) "Undefined" "OverrideRootScale" null (* (`KismetMathLibrary.Normal` (- (+ (`SceneComponent.K2_GetComponentLocation` `player camera`) (* (`SceneComponent.GetForwardVector` `player camera`) 10000.0)) _returnvalue)) (`self.get volacity`)) null)
      (`|SpawnActorFromClass` "/Game/bullet/bp_muzz.bp_muzz_C" (`KismetMathLibrary.MakeTransform` _returnvalue) "Undefined" "OverrideRootScale" null null))))

(fn `Fire Rate`
  (returns (Output_Get :type "Float (double-precision)"))
  (bind _output_get (set `self.FireRate` 1.0))
  (return _output_get))

(fn `Get interaction text`
  (returns (text :type Text))
  (return (`parent.Get interaction text`)))

(fn `get volacity`
  (returns (Output_Get :type "Float (double-precision)"))
  (return 0.0))

(fn `set gun state`
  (params (`New gun state` :type "/Game/items/guns/egunstate Enum" :default "NewEnumerator0"))
  (bind _skeletalmesh (`self.SkeletalMesh`))
  (bind _skeletalmesh_2 (`self.SkeletalMesh`))
  (bind _output_get (set `self.Gun State` `New gun state`))
  (switch `/Game/items/guns/egunstate` _output_get
    (:`NewEnumerator0`
      (`PrimitiveComponent.SetCollisionProfileName` (`self.Sphere`) "OverlapAllDynamic" true)
      (`PrimitiveComponent.SetSimulatePhysics` _skeletalmesh_2 true)
      (`PrimitiveComponent.SetCollisionProfileName` _skeletalmesh_2 "DroppedGun" true))
    (:`NewEnumerator1`
      (`PrimitiveComponent.SetCollisionProfileName` (`self.Sphere`) "NoCollision" true)
      (`PrimitiveComponent.SetSimulatePhysics` _skeletalmesh false)
      (`PrimitiveComponent.SetSimulatePhysics` (`self.Sphere`) false)
      (`PrimitiveComponent.SetCollisionProfileName` _skeletalmesh "NoCollision" true)
      (`SceneComponent.ResetRelativeTransform` (`self.SkeletalMesh`)))))

(fn `UserConstructionScript`
  (`parent.UserConstructionScript`))