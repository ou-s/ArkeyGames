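; Projectile bullet actor that flies at a set velocity and explodes on contact.
; BeginPlay copies its Velocity variable into ProjectileMovement, and a fire input press matches its rotation to the Ue4Asp actor.
; Any sphere overlap destroys the bullet, flags BulletHit and spawns a half-scale explosion effect at its location, owned by the overlapped actor.
; A Delay on Tick destroys the bullet after a few seconds as a lifetime limit.
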(event `self.ReceiveBeginPlay`
  (set `MovementComponent.Velocity` (`self.velocity`) (`self.ProjectileMovement`)))

(event `self.Sphere.OnComponentBeginOverlap`
  (params (OverlappedComponent :type "PrimitiveComponent Object Reference") (OtherActor :type "Actor Object Reference") (OtherComp :type "PrimitiveComponent Object Reference") (OtherBodyIndex :type Integer) (bFromSweep :type Boolean) (SweepResult :type "HitResult Structure (by ref)"))
  (`KismetSystemLibrary.PrintString` "dertoyed")
  (`|ExecutionSequence`
    (:`then_0`
      (`self.K2_DestroyActor`)
      (set `self.bullet hit` true))
    (:`then_1`
      (`|SpawnActorFromClass` "/Game/StarterContent/Blueprints/Blueprint_Effect_Explosion.Blueprint_Effect_Explosion_C" (`KismetMathLibrary.MakeTransform` (`self.bulet loaction`) (struct) (0.5 0.5 0.5)) "AlwaysSpawn" "OverrideRootScale" OtherActor null))))

(event `InputAction|fire`
  (params (Key :type "Key Structure"))
  (:`Pressed`
    (`self.K2_SetActorRotation` (`self.K2_GetActorRotation` (`self.ue4 asp`)))))

(event `self.ReceiveTick`
  (params (DeltaSeconds :type "Float (single-precision)"))
  (`KismetSystemLibrary.Delay` 3.0)
  (`self.K2_DestroyActor`))

(fn `bulet loaction`
  (returns (`actor location` :type "Vector Structure"))
  (return (`self.K2_GetActorLocation`)))

(fn `UserConstructionScript`)